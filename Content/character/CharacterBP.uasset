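; Player character Blueprint that handles walking and camera look through input axis events.
; The two camera axes feed controller yaw and pitch, while four WASD axes each call AddMovementInput.
; All four movement axes share the same direction: the forward vector of control-rotation pitch with yaw zeroed, so movement ignores camera heading and only axis scale distinguishes them.
; BeginPlay, overlap, Tick and the construction script are empty.
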(event `InputAxis|Поворот камеры| X | Ходьба`
  (params (AxisValue :type "Float (single-precision)"))
  (`self.AddControllerYawInput` AxisValue))

(event `InputAxis|Поворот камеры| Y | Ходьба`
  (params (AxisValue :type "Float (single-precision)"))
  (`self.AddControllerPitchInput` AxisValue))

(event `InputAxis|Вперёд | Ходьба`
  (params (AxisValue :type "Float (single-precision)"))
  ;[1 1 1] WASD
  (`self.AddMovementInput` (`KismetMathLibrary.GetForwardVector` (`KismetMathLibrary.MakeRotator` 0.0 (.pitch (`self.GetControlRotation`)))) AxisValue))

(event `InputAxis|Влево | Ходьба`
  (params (AxisValue :type "Float (single-precision)"))
  ;[1 1 1] WASD
  (`self.AddMovementInput` (`KismetMathLibrary.GetForwardVector` (`KismetMathLibrary.MakeRotator` 0.0 (.pitch (`self.GetControlRotation`)))) AxisValue))

(event `InputAxis|Вправо | Ходьба`
  (params (AxisValue :type "Float (single-precision)"))
  ;[1 1 1] WASD
  (`self.AddMovementInput` (`KismetMathLibrary.GetForwardVector` (`KismetMathLibrary.MakeRotator` 0.0 (.pitch (`self.GetControlRotation`)))) AxisValue))

(event `InputAxis|Назад | Ходьба`
  (params (AxisValue :type "Float (single-precision)"))
  ;[1 1 1] WASD
  (`self.AddMovementInput` (`KismetMathLibrary.GetForwardVector` (`KismetMathLibrary.MakeRotator` 0.0 (.pitch (`self.GetControlRotation`)))) AxisValue))

(fn `UserConstructionScript`)